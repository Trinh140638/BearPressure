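; Game mode Blueprint for BearPressure that runs a timed round and tracks the player's score.
; On BeginPlay it shows the HUD and plays the GameTime timeline, which writes the truncated track value to CurrentTime.
; When the timeline finishes, it adds the game over widget and shows the mouse cursor.
; The MailBoxHit event adds MailBoxPoints to CurrentScore and prints a debug string.
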(event `self.ReceiveBeginPlay`
  (bind _returnvalue (`|CreateWidget` "/Game/BearPressure/HUD/UI_HUD.UI_HUD_C" (`GameplayStatics.GetPlayerController` 0)))
  (`UserWidget.AddToViewport` _returnvalue 0)
  (bind (_direction _newtrack_0) (`Timeline|GameTime`)
    (:`Update`
      (set `self.CurrentTime` (`KismetMathLibrary.FTrunc` _newtrack_0)))
    (:`Finished`
      (bind _returnvalue_2 (`|CreateWidget` "/Game/BearPressure/HUD/UI_GameOver.UI_GameOver_C" (`GameplayStatics.GetPlayerController` 0)))
      (`UserWidget.AddToViewport` _returnvalue_2 0)
      (set `PlayerController.bShowMouseCursor` true (`GameplayStatics.GetPlayerController` 0)))))

(event `MailBoxHit`
  (set `self.CurrentScore` (+ (`self.CurrentScore`) (`self.MailBoxPoints`)))
  (`KismetSystemLibrary.PrintString` "Hello"))

(fn `UserConstructionScript`)
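; Objective detector actor that pulses controller rumble at a rate set by the player's proximity to an objective.
; BeginPlay caches the last BP_ObjectiveTest actor found and starts a looping ScanForObjective timer.
; Each scan measures XY-only distance, picks one of four range-based frequencies, plays force feedback and resets its own timer to that interval.
; Beyond far range it keeps scanning without rumbling; debug prints remain.
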(event `self.ReceiveBeginPlay`
  ;[0.3545 1 0.2159] Initialization: Find objective location, Spawn forcefeedbackcomponent (rumble), and start the rumble function with a looping timer
  (`self.NewObjective`)
  (`KismetSystemLibrary.K2_SetTimer` self "ScanForObjective" (`self.RumbleFrequency`) true))

(event `NewObjective`
  ;[1 0.349 0] NewObjective event: used to find location of new objective
  (bind _outactors (`GameplayStatics.GetAllActorsOfClass` "/Game/BearPressure/BP/Rumble/BP_ObjectiveTest.BP_ObjectiveTest_C"))
  (for _array_element _outactors
    (set `self.BP_ObjectiveActor` _array_element)))

(event `Rumble`
  ;[1 0.349 0] Rumble event: activate or edit the rumble function
  (`KismetSystemLibrary.K2_SetTimer` self "ControllerRumble" (`self.RumbleFrequency`) true))

(fn `ControllerRumble`
  (`PlayerController.ClientPlayForceFeedback` (`GameplayStatics.GetPlayerController` 0) "/Game/BearPressure/BP/Rumble/BP_ControllerRumble.BP_ControllerRumble" false false "None"))

(fn `ScanForObjective`
  (bind (_returnvalue_x _returnvalue_y) (`KismetMathLibrary.BreakVector` (- (`self.K2_GetActorLocation` (`GameplayStatics.GetPlayerPawn` 0)) (`self.K2_GetActorLocation` (`self.BP_ObjectiveActor`)))))
  (bind _returnvalue (`KismetMathLibrary.VSize` (`KismetMathLibrary.MakeVector` _returnvalue_x _returnvalue_y)))
  ;[1 1 1] Detect distance to the objective (only using X and Y location)
  (`KismetSystemLibrary.PrintString` (`KismetStringLibrary.Conv_DoubleToString` _returnvalue))
  (set `self.ObjectiveDistance` _returnvalue)
  ;[1 1 1] Figure out what range the player is in
  (if (<= (`self.ObjectiveDistance`) (`self.VeryNearDistance`))
    (bind _output_get (set `self.RumbleFrequency` (`self.VeryNearRumbleFrequency`)))
    (`KismetSystemLibrary.PrintString` (`KismetStringLibrary.Conv_DoubleToString` _output_get))
    ;[1 1 1] Activate controller rumble
    (`self.ControllerRumble` :!label _label)
    (`KismetSystemLibrary.K2_SetTimer` self "ScanForObjective" (`self.RumbleFrequency`) true)
    (elif (<= (`self.ObjectiveDistance`) (`self.NearDistance`))
      (bind _output_get_2 (set `self.RumbleFrequency` (`self.NearRumbleFrequency`)))
      (`KismetSystemLibrary.PrintString` (`KismetStringLibrary.Conv_DoubleToString` _output_get_2))
      (goto _label)
      (elif (<= (`self.ObjectiveDistance`) (`self.MediumDistance`))
        (bind _output_get_3 (set `self.RumbleFrequency` (`self.MediumRumbleFrequency`)))
        (`KismetSystemLibrary.PrintString` (`KismetStringLibrary.Conv_DoubleToString` _output_get_3))
        (goto _label)
        (elif (<= (`self.ObjectiveDistance`) (`self.FarDistance`))
          (bind _output_get_4 (set `self.RumbleFrequency` (`self.FarRumbleFrequency`)))
          (`KismetSystemLibrary.PrintString` (`KismetStringLibrary.Conv_DoubleToString` _output_get_4))
          (goto _label))))))

(fn `UserConstructionScript`)
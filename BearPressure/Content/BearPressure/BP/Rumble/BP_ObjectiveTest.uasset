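; BP_ObjectiveTest is a mailbox delivery objective with a bobbing arrow, completed through its Dashing event.
; BeginPlay notifies BP_ObjectiveDetector of the spawn and loops two latent MoveComponentTo calls on the arrow.
; Dashing removes the arrow, reports MailBoxHit to BP_GameMode, and animates the lid by timeline before requesting the next objective and destroying itself.
; Its HasBeenHit guard never latches, as the flag is set to false.
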(event `/Game/BearPressure/Character/BPI_PlayerInteractions.Dashing`
  (if (not (`self.HasBeenHit`))
    (`|ExecutionSequence`
      (:`then_0`
        (set `self.HasBeenHit` false))
      (:`then_1`
        (`ActorComponent.K2_DestroyComponent` (`self.ObjectiveArrow`)))
      (:`then_2`
        (bind _outactors (`GameplayStatics.GetAllActorsOfClass` "/Game/BearPressure/BP/BP_GameMode.BP_GameMode_C"))
        (for _array_element _outactors
          (bind _asbp_game_mode (cast `/Game/BearPressure/BP/BP_GameMode` _array_element))
          (`/Game/BearPressure/BP/BP_GameMode.MailBoxHit` _asbp_game_mode)))
      (:`then_3`
        (bind (_direction _newtrack_0) (`Timeline|MailDelivered`)
          (:`Update`
            (`SceneComponent.K2_SetRelativeRotation` (`self.MailLidPivot`) (`KismetMathLibrary.MakeRotator` 0.0 _newtrack_0) false false))
          (:`Finished`
            (bind _outactors_2 (`GameplayStatics.GetAllActorsOfClass` "/Game/BearPressure/BP/Rumble/BP_ObjectiveDetector.BP_ObjectiveDetector_C"))
            (`/Game/BearPressure/BP/Rumble/BP_ObjectiveDetector.Spawn Objective` (`|GetArrayItem` _outactors_2))
            (`self.K2_DestroyActor`)))))))

(event `self.ReceiveBeginPlay`
  (bind _objectivearrow (`self.ObjectiveArrow`))
  (set `self.ArrowStartLoc` (`SceneComponent.K2_GetComponentLocation` (`self.ObjectiveArrow`)))
  (bind _outactors (`GameplayStatics.GetAllActorsOfClass` "/Game/BearPressure/BP/Rumble/BP_ObjectiveDetector.BP_ObjectiveDetector_C"))
  (`/Game/BearPressure/BP/Rumble/BP_ObjectiveDetector.Objective Spawned` (`|GetArrayItem` _outactors))
  (`KismetSystemLibrary.PrintString` (`KismetStringLibrary.Concat_StrStr` "Objective spawned at " (`KismetStringLibrary.Conv_VectorToString` (`self.K2_GetActorLocation`))))
  (`KismetSystemLibrary.MoveComponentTo` _objectivearrow (+ (`self.ArrowStartLoc`) (0.0 0.0 -30.0)) (struct) false false 0.4 :!label _label)
  (`KismetSystemLibrary.MoveComponentTo` _objectivearrow (+ (`self.ArrowStartLoc`) (0.0 0.0 30.0)) (struct) false false 0.4)
  (goto _label))

(fn `UserConstructionScript`)
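; Core movement Blueprint for the Pigear character, with camera-relative walking and a self-centering camera.
; Forward and Right axes add movement along the CameraCenter vectors.
; On Tick, the mesh snaps to the input direction once input passes a small deadzone.
; With camera input idle, CameraCenter eases behind the mesh, faster as misalignment grows, but holds when the mesh faces mostly back toward the camera.
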(event `self.ReceiveTick`
  (params (DeltaSeconds :type "Float (single-precision)"))
  (bind _returnvalue (`SceneComponent.K2_GetComponentRotation` (`self.Mesh`)))
  (bind _returnvalue_2 (`SceneComponent.K2_GetComponentRotation` (`self.Camera Center`)))
  (bind _returnvalue_3 (`KismetMathLibrary.Dot_VectorVector` (`KismetMathLibrary.Conv_RotatorToVector` _returnvalue_2) (`KismetMathLibrary.Conv_RotatorToVector` _returnvalue)))
  (`|ExecutionSequence`
    (:`then_0`
      (if (> (+ (`KismetMathLibrary.Abs` (`self.GetInputAxisValue`)) (`KismetMathLibrary.Abs` (`self.GetInputAxisValue`))) 0.25)
        (`SceneComponent.K2_SetWorldRotation` (`self.Mesh`) (`KismetMathLibrary.FindLookAtRotation` (0.0 0.0 0.0) (+ (* (`SceneComponent.GetForwardVector` (`self.Camera Center`)) (`self.GetInputAxisValue`)) (* (`SceneComponent.GetRightVector` (`self.Camera Center`)) (`self.GetInputAxisValue`)))) false false)))
    (:`then_1`
      (if (and (`KismetMathLibrary.NearlyEqual_FloatFloat` (+ (`KismetMathLibrary.Abs` (`self.GetInputAxisValue`)) (`KismetMathLibrary.Abs` (`self.GetInputAxisValue`))) 0.0 0.01) (> _returnvalue_3 -0.65))
        (`SceneComponent.K2_SetWorldRotation` (`self.Camera Center`) (`KismetMathLibrary.RInterpTo` _returnvalue_2 _returnvalue (`GameplayStatics.GetWorldDeltaSeconds`) (`KismetMathLibrary.MapRangeUnclamped` _returnvalue_3 1.0 0.0 0.25 0.6)) false false)))))

(event `InputAxis|Right` :consume false
  (params (AxisValue :type "Float (single-precision)"))
  (`self.AddMovementInput` (`SceneComponent.GetRightVector` (`self.Camera Center`)) AxisValue))

(event `InputAxis|Forward` :consume false
  (params (AxisValue :type "Float (single-precision)"))
  (`self.AddMovementInput` (`SceneComponent.GetForwardVector` (`self.Camera Center`)) AxisValue))

(fn `UserConstructionScript`
  (`parent.UserConstructionScript`))
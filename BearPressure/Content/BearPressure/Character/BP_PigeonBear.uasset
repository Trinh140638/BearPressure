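; BP_PigeonBear is a player-controlled character with camera-relative movement.
; The Camera_X axis yaws the CameraCenter component, whose forward and right vectors set the direction for the Forward and Right movement inputs.
; On Tick, when combined input magnitude passes a small dead zone, the Mesh instantly turns to face the camera-relative input direction, independent of camera yaw input otherwise.
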(event `InputAxis|Camera_X`
  (params (AxisValue :type "Float (single-precision)"))
  (`SceneComponent.K2_AddRelativeRotation` (`self.Camera Center`) (`KismetMathLibrary.MakeRotator` 0.0 0.0 AxisValue) false false))

(event `self.ReceiveTick`
  (params (DeltaSeconds :type "Float (single-precision)"))
  (if (> (+ (`KismetMathLibrary.Abs` (`self.GetInputAxisValue`)) (`KismetMathLibrary.Abs` (`self.GetInputAxisValue`))) 0.25)
    (`SceneComponent.K2_SetWorldRotation` (`self.Mesh`) (`KismetMathLibrary.FindLookAtRotation` (0.0 0.0 0.0) (+ (* (`SceneComponent.GetForwardVector` (`self.Camera Center`)) (`self.GetInputAxisValue`)) (* (`SceneComponent.GetRightVector` (`self.Camera Center`)) (`self.GetInputAxisValue`)))) false false)))

(event `InputAxis|Forward`
  (params (AxisValue :type "Float (single-precision)"))
  (`self.AddMovementInput` (`SceneComponent.GetForwardVector` (`self.Camera Center`)) AxisValue))

(event `InputAxis|Right`
  (params (AxisValue :type "Float (single-precision)"))
  (`self.AddMovementInput` (`SceneComponent.GetRightVector` (`self.Camera Center`)) AxisValue))

(fn `UserConstructionScript`)
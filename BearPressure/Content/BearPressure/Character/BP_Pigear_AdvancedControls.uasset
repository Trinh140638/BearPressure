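; Pigear player character Blueprint adding stamina-limited flapping, gliding and a ground dash, with a stamina bar widget created on BeginPlay.
; A downward line trace splits Jump into a ground launch or a stamina-costing flap, and holding it sets Gliding.
; Tick regenerates stamina and relaunches the character forward and down while gliding.
; Dash traces forward, notifies BPI_PlayerInteractions actors, then timeline-lerps the character behind a cooldown gate.
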(event `self.ReceiveBeginPlay`
  (`parent.ReceiveBeginPlay`)
  (bind _returnvalue (`|CreateWidget` "/Game/BearPressure/HUD/WB_StaminaBar.WB_StaminaBar_C"))
  (`UserWidget.AddToPlayerScreen` _returnvalue 0))

(event `CameraFOVFire`
  ;[1 1 1] Rubbish
  (if (not (`self.FovFired`))
    (`|ExecutionSequence`
      (:`then_0`
        (set `self.FovFired` true))
      (:`then_1`
        (bind _outactors (`GameplayStatics.GetAllActorsOfClass` "/Game/BearPressure/Character/BP_Pigear_Camera.BP_Pigear_Camera_C"))
        (for _array_element _outactors
          (`self.StartFlying` _array_element)
          (`KismetSystemLibrary.Delay` 1.0)
          (if (not (`self.ButtonFired`))
            (`self.CameraFOVLow`)))))))

(event `self.ReceiveTick`
  (params (DeltaSeconds :type "Float (single-precision)"))
  (bind _stamina_meter (`self.Stamina Meter`))
  (`parent.ReceiveTick` DeltaSeconds)
  (`|ExecutionSequence`
    (:`then_0`
      (if (< (`self.Stamina Meter`) 10.0)
        (`|VariableSetRef` _stamina_meter (+ _stamina_meter 0.025))))
    (:`then_1`
      (if (`self.Gliding`)
        (`self.LaunchCharacter` (+ (* (`SceneComponent.GetForwardVector` (`self.Mesh`)) 900.0) (0.0 0.0 -320.0)) true true)))))

(event `CameraFOVLow`
  ;[1 1 1] Rubbish
  (bind _outactors (`GameplayStatics.GetAllActorsOfClass` "/Game/BearPressure/Character/BP_Pigear_Camera.BP_Pigear_Camera_C"))
  (for _ _outactors
    (`self.StopFlying`)))

(event `InputAction|Jump`
  (params (Key :type "Key Structure")))

(event `InputAction|Jump`
  (params (Key :type "Key Structure"))
  (:`Pressed`
    (`self.Check if Grounded`
      (:`Grounded`
        (`self.Jumped`)
        (`self.LaunchCharacter` (`KismetMathLibrary.MakeVector` 0.0 0.0 (`self.Jump Height (On Ground)`)))
        (`KismetSystemLibrary.Delay` 0.5)
        (set `self.Gliding` (>= (`PlayerController.GetInputKeyTimeDown` (`GameplayStatics.GetPlayerController` 0) Key) 0.45)))
      (:`Not Grounded`
        (if (>= (`self.Stamina Meter`) 1.0)
          (`self.Flapped`)
          (`self.LaunchCharacter` (+ (* (`SceneComponent.GetForwardVector` (`self.Mesh`)) (`self.Flap Forward Push`)) (`KismetMathLibrary.MakeVector` 0.0 0.0 (`self.Flap Height Increase`))) true true)
          (`/Engine/EditorBlueprintResources/StandardMacros.DecrementFloat` (`self.Stamina Meter`)
            (:`  `
              _)))
        (`KismetSystemLibrary.RetriggerableDelay` 0.25)
        (set `self.Gliding` (>= (`PlayerController.GetInputKeyTimeDown` (`GameplayStatics.GetPlayerController` 0) Key) 0.2)))))
  (:`Released`
    (if (`self.Gliding`)
      (set `self.Gliding` false))))

(event `InputAction|Dash`
  (params (Key :type "Key Structure"))
  (bind _returnvalue (`self.K2_GetActorLocation`))
  (:`Pressed`
    (`self.Check if Grounded`
      (:`Grounded`
        (`/Engine/EditorBlueprintResources/StandardMacros.Gate` false :!label _label
          (:`Exit`
            (`|ExecutionSequence`
              (:`then_0`
                (goto _label :!via `Close`))
              (:`then_1`
                (`self.DoingTheDash`)
                (bind _outhit (`KismetSystemLibrary.LineTraceSingle` :`Start` _returnvalue :`End` (+ _returnvalue (* (`SceneComponent.GetForwardVector` (`self.Mesh`)) (`self.Dash Distance`))) :`TraceChannel` "TraceTypeQuery1" :`DrawDebugType` "ForDuration"))
                (`|ExecutionSequence`
                  (:`then_0`
                    (bind _returnvalue_2 (`KismetSystemLibrary.DoesImplementInterface` (`.HitActor` (`GameplayStatics.BreakHitResult` _outhit)) "/Game/BearPressure/Character/BPI_PlayerInteractions.BPI_PlayerInteractions_C"))
                    (if _returnvalue_2
                      (message `/Game/BearPressure/Character/BPI_PlayerInteractions.Dashing` (`.HitActor` (`GameplayStatics.BreakHitResult` _outhit)))))
                  (:`then_1`
                    (bind (_direction _newtrack_0) (`Timeline|Timeline_0_0` :!via `PlayFromStart`)
                      (:`Update`
                        (`self.K2_SetActorLocation` (`KismetMathLibrary.VLerp` (`.TraceStart` (`GameplayStatics.BreakHitResult` _outhit)) (select `bool` (and (`GameplayStatics.BreakHitResult` _outhit) _returnvalue_2) :`false` (`.TraceEnd` (`GameplayStatics.BreakHitResult` _outhit)) :`true` (`.Location` (`GameplayStatics.BreakHitResult` _outhit))) _newtrack_0) true))
                      (:`Finished`
                        (`KismetSystemLibrary.Delay` (`self.Dash Cooldown`))
                        (goto _label :!via `Open`)))))))))))))

(fn `UserConstructionScript`
  (`parent.UserConstructionScript`)
  (set `CharacterMovementComponent.MaxWalkSpeed` (`self.Walking Speed`) (`self.CharacterMovement`)))
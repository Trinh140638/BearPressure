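; Bp_Car is a hazard car that drives forward at constant speed and kills BP_Pigear_Jews actors it overlaps.
; Tick moves it along its forward vector with a sweep, and a lifespan set on BeginPlay removes it after a fixed time.
; On overlap it passes its right vector and location to the victim's Kill.
; A Dashing event spawns an explosion above the car and destroys it.
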(event `self.ReceiveActorBeginOverlap`
  (params (OtherActor :type "Actor Object Reference"))
  (bind _asbp_pigear_jews (cast `/Game/BearPressure/Character/BP_Pigear_Jews` OtherActor))
  (`/Game/BearPressure/Character/BP_Pigear_Jews.Kill` _asbp_pigear_jews (`self.GetActorRightVector`) (`self.K2_GetActorLocation`)))

(event `self.ReceiveBeginPlay`
  (`self.SetLifeSpan` 37.0))

(event `self.ReceiveTick`
  (params (DeltaSeconds :type "Float (single-precision)"))
  (`self.K2_SetActorLocation` (+ (`self.K2_GetActorLocation`) (* (`KismetMathLibrary.Normal` (`self.GetActorForwardVector`)) (* DeltaSeconds 600.0))) true))

(event `/Game/BearPressure/Character/BPI_PlayerInteractions.Dashing`
  (`GameplayStatics.SpawnEmitterAtLocation` "/Game/BearPressure/Art/Explosion.Explosion" (+ (`self.K2_GetActorLocation`) (0.0 0.0 100.0)))
  (`self.K2_DestroyActor`))

(fn `UserConstructionScript`)
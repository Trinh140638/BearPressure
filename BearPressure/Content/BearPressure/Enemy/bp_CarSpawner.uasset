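; Car spawner that sends recurring waves of Bp_Car traffic onto the roads of the generated map.
; Each Tick finds Bp_MapGenerator, and a DoOnce gates a delayed wave built from its road points, road length and grid size.
; X roads spawn first and Y roads five seconds later, with opposing cars at both ends and random CarTypes meshes.
; The Y loop resets the DoOnce, so waves repeat.
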(event `self.ReceiveTick`
  (params (DeltaSeconds :type "Float (single-precision)"))
  (bind _car_types (`self.Car Types`))
  (bind _car_types_2 (`self.Car Types`))
  (bind _map_gen (`self.Map Gen`))
  (bind _map_gen_2 (`self.Map Gen`))
  (bind _map_gen_3 (`self.Map Gen`))
  (bind _map_gen_4 (`self.Map Gen`))
  (bind _car_types_3 (`self.Car Types`))
  (bind _car_types_4 (`self.Car Types`))
  (bind _road_lenght (`/Game/BearPressure/TileSystem/Bp_MapGenerator.Road Lenght` _map_gen_4))
  (bind _road_lenght_2 (`/Game/BearPressure/TileSystem/Bp_MapGenerator.Road Lenght` _map_gen))
  (bind _returnvalue (* (* _road_lenght 2) -1))
  (bind _returnvalue_2 (* (* _road_lenght_2 2) -1))
  (bind _outactors (`GameplayStatics.GetAllActorsOfClass` "/Game/BearPressure/TileSystem/Bp_MapGenerator.Bp_MapGenerator_C"))
  (set `self.Map Gen` (`|GetArrayItem` _outactors))
  (`/Engine/EditorBlueprintResources/StandardMacros.DoOnce` false :!label _label
    (:`Completed`
      (`KismetSystemLibrary.Delay` 10.0)
      (`|ExecutionSequence`
        (:`then_0`
          (for _array_element (`/Game/BearPressure/TileSystem/Bp_MapGenerator.Road points X` _map_gen)
            (bind _returnvalue_3 (`KismetMathLibrary.MakeVector` (`KismetMathLibrary.Conv_IntToDouble` (- (+ (* _array_element _road_lenght_2) _returnvalue_2) 350)) (`KismetMathLibrary.Conv_IntToDouble` (- _returnvalue_2 _road_lenght_2)) 0.0))
            (bind _returnvalue_4 (`|SpawnActorFromClass` "/Game/BearPressure/Enemy/Bp_Car.Bp_Car_C" (`KismetMathLibrary.MakeTransform` _returnvalue_3 (struct :`Yaw` 90.0)) "AlwaysSpawn" "OverrideRootScale" null null))
            (`StaticMeshComponent.SetStaticMesh` (`/Game/BearPressure/Enemy/Bp_Car.StaticMesh` _returnvalue_4) (`|GetArrayItem` _car_types_3 (`KismetMathLibrary.RandomInteger` (`KismetArrayLibrary.Array_Length` _car_types_3))))
            (bind _returnvalue_5 (`|SpawnActorFromClass` "/Game/BearPressure/Enemy/Bp_Car.Bp_Car_C" (`KismetMathLibrary.MakeTransform` (`KismetMathLibrary.MakeVector` (+ (.x _returnvalue_3) 700.0) (+ (.y _returnvalue_3) (`KismetMathLibrary.Conv_IntToDouble` (* (`/Game/BearPressure/TileSystem/Bp_MapGenerator.Road Lenght` _map_gen_3) (* (`/Game/BearPressure/TileSystem/Bp_MapGenerator.Amount of roads in a row` _map_gen_3) 2)))) 0.0) (struct :`Yaw` -90.0)) "AlwaysSpawn" "OverrideRootScale" null null))
            (`StaticMeshComponent.SetStaticMesh` (`/Game/BearPressure/Enemy/Bp_Car.StaticMesh` _returnvalue_5) (`|GetArrayItem` _car_types_2 (`KismetMathLibrary.RandomInteger` (`KismetArrayLibrary.Array_Length` _car_types_2))))))
        (:`then_1`
          (`KismetSystemLibrary.Delay` 5.0)
          (for _array_element_2 (`/Game/BearPressure/TileSystem/Bp_MapGenerator.Road Points Y` _map_gen_4)
            (bind _returnvalue_6 (`KismetMathLibrary.MakeVector` (`KismetMathLibrary.Conv_IntToDouble` (- _returnvalue _road_lenght)) (`KismetMathLibrary.Conv_IntToDouble` (- (+ (* _array_element_2 _road_lenght) _returnvalue) -350)) 0.0))
            (bind _returnvalue_7 (`|SpawnActorFromClass` "/Game/BearPressure/Enemy/Bp_Car.Bp_Car_C" (`KismetMathLibrary.MakeTransform` _returnvalue_6) "AlwaysSpawn" "OverrideRootScale" null null))
            (`StaticMeshComponent.SetStaticMesh` (`/Game/BearPressure/Enemy/Bp_Car.StaticMesh` _returnvalue_7) (`|GetArrayItem` _car_types_4 (`KismetMathLibrary.RandomInteger` (`KismetArrayLibrary.Array_Length` _car_types_4))))
            (bind _returnvalue_8 (`|SpawnActorFromClass` "/Game/BearPressure/Enemy/Bp_Car.Bp_Car_C" (`KismetMathLibrary.MakeTransform` (`KismetMathLibrary.MakeVector` (+ (.x _returnvalue_6) (`KismetMathLibrary.Conv_IntToDouble` (* (`/Game/BearPressure/TileSystem/Bp_MapGenerator.Road Lenght` _map_gen_2) (* (`/Game/BearPressure/TileSystem/Bp_MapGenerator.Amount of roads in a row` _map_gen_2) 2)))) (+ (.y _returnvalue_6) -700.0) 0.0) (struct :`Yaw` 180.0)) "AlwaysSpawn" "OverrideRootScale" null null))
            (`StaticMeshComponent.SetStaticMesh` (`/Game/BearPressure/Enemy/Bp_Car.StaticMesh` _returnvalue_8) (`|GetArrayItem` _car_types (`KismetMathLibrary.RandomInteger` (`KismetArrayLibrary.Array_Length` _car_types))))
            (goto _label :!via `Reset`)))))))

(fn `UserConstructionScript`)
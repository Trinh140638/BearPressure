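; Map generator actor that builds a random tile-based city grid of roads, crossroads and house tiles at BeginPlay.
; It picks random even grid lines per axis, spawns roads along them, crossroads at intersections and road pieces in gaps, then fills the rest with houses.
; Each tile gets a random mesh from its array.
; Pressing V destroys tiles and objectives, has BP_ObjectiveDetector spawn an objective, then rebuilds.
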(event `self.ReceiveBeginPlay`
  (`self.EnableInput` (`GameplayStatics.GetPlayerController` 0))
  (`self.Create Road Points` :!label _label)
  (for _array_element (`self.Road points X`)
    (`self.Spawn Road` _array_element true "/Game/BearPressure/TileSystem/Sm_Road.Sm_Road_C"))
  (for _array_element_2 (`self.Road Points Y`)
    (`self.Spawn Road` _array_element_2 false "/Game/BearPressure/TileSystem/Sm_Road.Sm_Road_C"))
  (`self.Spawn Cross Roads`)
  (`self.Spawn Road Gabs`)
  (`self.Spawn Building Tiles`))

(event `Key|V`
  (params (Key :type "Key Structure"))
  (:`Pressed`
    (`self.Re-Generate Level`)
    (goto _label)))

(fn `Create Road Points`
  (bind _current_number (`self.Current number`))
  (for _index (range 2)
    (for _ (range 1 (+ (`self.Road spawn rate`) 1))
      (bind _output_get (set `self.Current number` (`KismetMathLibrary.RandomInteger` (* (`self.Amount of roads in a row`) 2))))
      (if (> (mod _output_get 2) 0)
        _
        (elif (== _index 0)
          (`KismetArrayLibrary.Array_AddUnique` (`self.Road points X`) _current_number)
          (else
            (`KismetArrayLibrary.Array_AddUnique` (`self.Road Points Y`) _current_number)))))))

(fn `Re-Generate Level`
  (bind _outactors (`GameplayStatics.GetAllActorsOfClass` "/Game/BearPressure/TileSystem/Sm_Road.Sm_Road_C"))
  (for _array_element _outactors
    (`self.K2_DestroyActor` _array_element))
  (bind _outactors_2 (`GameplayStatics.GetAllActorsOfClass` "/Game/BearPressure/TileSystem/Sm_CrossRoad.Sm_CrossRoad_C"))
  (for _array_element_2 _outactors_2
    (`self.K2_DestroyActor` _array_element_2))
  (bind _outactors_3 (`GameplayStatics.GetAllActorsOfClass` "/Game/BearPressure/TileSystem/Sm_HouseTile.Sm_HouseTile_C"))
  (for _array_element_3 _outactors_3
    (`self.K2_DestroyActor` _array_element_3))
  (bind _outactors_4 (`GameplayStatics.GetAllActorsOfClass` "/Game/BearPressure/BP/Rumble/BP_ObjectiveTest.BP_ObjectiveTest_C"))
  (for _array_element_4 _outactors_4
    (`self.K2_DestroyActor` _array_element_4))
  (bind _outactors_5 (`GameplayStatics.GetAllActorsOfClass` "/Game/BearPressure/BP/Rumble/BP_ObjectiveDetector.BP_ObjectiveDetector_C"))
  (`/Game/BearPressure/BP/Rumble/BP_ObjectiveDetector.Spawn Objective` (`|GetArrayItem` _outactors_5))
  (`KismetArrayLibrary.Array_Clear` (`self.Road points X`))
  (`KismetArrayLibrary.Array_Clear` (`self.Road Points Y`))
  (return))

(fn `Spawn Building Tiles`
  (bind _road_lenght (`self.Road Lenght`))
  (bind _road_lenght_2 (`self.Road Lenght`))
  (bind _house_tiles (`self.House Tiles`))
  (bind _house_tiles_2 (`self.House Tiles`))
  (bind _returnvalue (* _road_lenght_2 2))
  (bind _returnvalue_2 (* _road_lenght 2))
  (bind _returnvalue_3 (+ (* (`self.Amount of roads in a row`) 2) 1))
  (`|ExecutionSequence`
    (:`then_0`
      (for _index (range (+ _returnvalue_3 1))
        (if (> (mod _index 2) 0)
          (for _index_2 (range (+ _returnvalue_3 1))
            (if (> (mod _index_2 2) 0)
              (bind (_returnvalue_x _returnvalue_y _returnvalue_z) (`KismetMathLibrary.BreakVector` (+ (`KismetMathLibrary.MakeVector` (`KismetMathLibrary.Conv_IntToDouble` (- (* _index_2 _road_lenght) _returnvalue_2))) (`KismetMathLibrary.MakeVector` (`KismetMathLibrary.Conv_IntToDouble` (* _returnvalue_2 -1)) (* _returnvalue_2 -1.5)))))
              (bind _returnvalue_4 (`|SpawnActorFromClass` "/Game/BearPressure/TileSystem/Sm_HouseTile.Sm_HouseTile_C" (`KismetMathLibrary.MakeTransform` (`KismetMathLibrary.MakeVector` _returnvalue_x (+ _returnvalue_y (`KismetMathLibrary.Conv_IntToDouble` (* (/ _index 2) _returnvalue_2))) _returnvalue_z)) "Undefined" "OverrideRootScale" null null))
              (`StaticMeshComponent.SetStaticMesh` (`StaticMeshActor.StaticMeshComponent` _returnvalue_4) (`|GetArrayItem` _house_tiles (`KismetMathLibrary.RandomInteger` (`KismetArrayLibrary.Array_Length` _house_tiles)))))))))
    (:`then_1`
      (`KismetArrayLibrary.Array_Clear` (`self.Temp Array`))
      (`KismetArrayLibrary.Array_Clear` (`self.Temp Array2`))
      (for _index_3 (range (+ (* (`self.Amount of roads in a row`) 2) 1))
        (if (not (> (mod _index_3 2) 0))
          (`|ExecutionSequence`
            (:`then_0`
              (if (not (`KismetArrayLibrary.Array_Contains` (`self.Road points X`) _index_3))
                (`KismetArrayLibrary.Array_AddUnique` (`self.Temp Array`) _index_3)))
            (:`then_1`
              (if (not (`KismetArrayLibrary.Array_Contains` (`self.Road Points Y`) _index_3))
                (`KismetArrayLibrary.Array_AddUnique` (`self.Temp Array2`) _index_3))))))
      (for _array_element (`self.Temp Array`)
        (`self.Spawn Road` _array_element true "/Game/BearPressure/TileSystem/Sm_HouseTile.Sm_HouseTile_C"))
      (for _array_element_2 (`self.Temp Array2`)
        (`self.Spawn Road` _array_element_2 false "/Game/BearPressure/TileSystem/Sm_HouseTile.Sm_HouseTile_C")))
    (:`then_2`
      (for _array_element_3 (`self.Temp Array`)
        (for _array_element_4 (`self.Temp Array2`)
          (bind (_returnvalue_x_2 _returnvalue_y_2 _returnvalue_z_2) (`KismetMathLibrary.BreakVector` (+ (`KismetMathLibrary.MakeVector` (`KismetMathLibrary.Conv_IntToDouble` (* _array_element_3 _road_lenght_2))) (`KismetMathLibrary.MakeVector` (`KismetMathLibrary.Conv_IntToDouble` (* _returnvalue -1)) (* _returnvalue -1.5)))))
          (bind _returnvalue_5 (`|SpawnActorFromClass` "/Game/BearPressure/TileSystem/Sm_HouseTile.Sm_HouseTile_C" (`KismetMathLibrary.MakeTransform` (`KismetMathLibrary.MakeVector` _returnvalue_x_2 (+ _returnvalue_y_2 (`KismetMathLibrary.Conv_IntToDouble` (+ _road_lenght_2 (* (/ _array_element_4 2) _returnvalue)))) _returnvalue_z_2)) "Undefined" "OverrideRootScale" null null))
          (`StaticMeshComponent.SetStaticMesh` (`StaticMeshActor.StaticMeshComponent` _returnvalue_5) (`|GetArrayItem` _house_tiles_2 (`KismetMathLibrary.RandomInteger` (`KismetArrayLibrary.Array_Length` _house_tiles_2)))))))))

(fn `Spawn Cross Roads`
  (bind _road_lenght (`self.Road Lenght`))
  (bind _crossroad_tiles (`self.CrossRoad Tiles`))
  (bind _returnvalue (* _road_lenght 2))
  (for _array_element (`self.Road points X`)
    (for _array_element_2 (`self.Road Points Y`)
      (bind (_returnvalue_x _returnvalue_y _returnvalue_z) (`KismetMathLibrary.BreakVector` (+ (`KismetMathLibrary.MakeVector` (`KismetMathLibrary.Conv_IntToDouble` (* _array_element _road_lenght))) (`KismetMathLibrary.MakeVector` (`KismetMathLibrary.Conv_IntToDouble` (* _returnvalue -1)) (* _returnvalue -1.5)))))
      (bind _returnvalue_2 (`|SpawnActorFromClass` "/Game/BearPressure/TileSystem/Sm_CrossRoad.Sm_CrossRoad_C" (`KismetMathLibrary.MakeTransform` (`KismetMathLibrary.MakeVector` _returnvalue_x (+ _returnvalue_y (`KismetMathLibrary.Conv_IntToDouble` (+ _road_lenght (* (/ _array_element_2 2) _returnvalue)))) _returnvalue_z)) "Undefined" "OverrideRootScale" null null))
      (`StaticMeshComponent.SetStaticMesh` (`StaticMeshActor.StaticMeshComponent` _returnvalue_2) (`|GetArrayItem` _crossroad_tiles (`KismetMathLibrary.RandomInteger` (`KismetArrayLibrary.Array_Length` _crossroad_tiles)))))))

(fn `Spawn Road`
  (params (`Grid number` :type Integer) (`Grid X` :type Boolean) (`Model to Spawn` :type "StaticMeshActor Class Reference"))
  (bind _road_lenght (`self.Road Lenght`))
  (bind _house_tiles (`self.House Tiles`))
  (bind _house_tiles_2 (`self.House Tiles`))
  (bind _road_tiles (`self.Road Tiles`))
  (bind _road_tiles_2 (`self.Road Tiles`))
  (bind _returnvalue (* _road_lenght 2))
  (bind _returnvalue_2 (`KismetMathLibrary.Conv_IntToDouble` (* `Grid number` _road_lenght)))
  (bind _returnvalue_3 (* _returnvalue -1.5))
  (bind _returnvalue_4 (* _returnvalue -1))
  (bind (_returnvalue_x _returnvalue_y _returnvalue_z) (`KismetMathLibrary.BreakVector` (+ (`KismetMathLibrary.MakeVector` _returnvalue_2) (`KismetMathLibrary.MakeVector` (`KismetMathLibrary.Conv_IntToDouble` _returnvalue_4) _returnvalue_3))))
  (bind (_returnvalue_x_2 _returnvalue_y_2 _returnvalue_z_2) (`KismetMathLibrary.BreakVector` (+ (`KismetMathLibrary.MakeVector` _returnvalue_3 (`KismetMathLibrary.Conv_IntToDouble` _returnvalue_4)) (`KismetMathLibrary.MakeVector` 0.0 _returnvalue_2))))
  (if `Grid X`
    (for _index (range (+ (`self.Amount of roads in a row`) 1))
      (bind _returnvalue_5 (`|SpawnActorFromClass` `Model to Spawn` (`KismetMathLibrary.MakeTransform` (`KismetMathLibrary.MakeVector` _returnvalue_x (+ _returnvalue_y (`KismetMathLibrary.Conv_IntToDouble` (* _index _returnvalue))) _returnvalue_z) (struct :`Yaw` 90.0)) "Undefined" "OverrideRootScale" null null))
      (if (== `Model to Spawn` "/Game/BearPressure/TileSystem/Sm_HouseTile.Sm_HouseTile_C")
        (`StaticMeshComponent.SetStaticMesh` (`StaticMeshActor.StaticMeshComponent` _returnvalue_5) (`|GetArrayItem` _house_tiles_2 (`KismetMathLibrary.RandomInteger` (`KismetArrayLibrary.Array_Length` _house_tiles_2))))
        (else
          (`StaticMeshComponent.SetStaticMesh` (`StaticMeshActor.StaticMeshComponent` _returnvalue_5) (`|GetArrayItem` _road_tiles (`KismetMathLibrary.RandomInteger` (`KismetArrayLibrary.Array_Length` _road_tiles)))))))
    (else
      (for _index_2 (range (+ (`self.Amount of roads in a row`) 1))
        (bind _returnvalue_6 (`|SpawnActorFromClass` `Model to Spawn` (`KismetMathLibrary.MakeTransform` (`KismetMathLibrary.MakeVector` (+ _returnvalue_x_2 (* _index_2 (`KismetMathLibrary.Conv_IntToDouble` _returnvalue))) _returnvalue_y_2 _returnvalue_z_2)) "Undefined" "OverrideRootScale" null null))
        (if (== `Model to Spawn` "/Game/BearPressure/TileSystem/Sm_HouseTile.Sm_HouseTile_C")
          (`StaticMeshComponent.SetStaticMesh` (`StaticMeshActor.StaticMeshComponent` _returnvalue_6) (`|GetArrayItem` _house_tiles (`KismetMathLibrary.RandomInteger` (`KismetArrayLibrary.Array_Length` _house_tiles))))
          (else
            (`StaticMeshComponent.SetStaticMesh` (`StaticMeshActor.StaticMeshComponent` _returnvalue_6) (`|GetArrayItem` _road_tiles_2 (`KismetMathLibrary.RandomInteger` (`KismetArrayLibrary.Array_Length` _road_tiles_2))))))))))

(fn `Spawn Road Gabs`
  (bind _road_lenght (`self.Road Lenght`))
  (bind _road_lenght_2 (`self.Road Lenght`))
  (bind _road_tiles (`self.Road Tiles`))
  (bind _road_tiles_2 (`self.Road Tiles`))
  (bind _returnvalue (* _road_lenght 2))
  (bind _returnvalue_2 (* _road_lenght_2 2))
  (`KismetArrayLibrary.Array_Clear` (`self.Temp Array`))
  (`|ExecutionSequence`
    (:`then_0`
      (for _index (range (+ (* (`self.Amount of roads in a row`) 2) 1))
        (`KismetArrayLibrary.Array_Clear` (`self.Temp Array`))
        (if (> (mod _index 2) 0)
          _
          (elif (not (`KismetArrayLibrary.Array_Contains` (`self.Road Points Y`) _index))
            (`KismetArrayLibrary.Array_Add` (`self.Temp Array`) _index)
            (for _array_element (`self.Road points X`)
              (for _array_element_2 (`self.Temp Array`)
                (bind (_returnvalue_x _returnvalue_y _returnvalue_z) (`KismetMathLibrary.BreakVector` (+ (`KismetMathLibrary.MakeVector` (`KismetMathLibrary.Conv_IntToDouble` (* _array_element _road_lenght_2))) (`KismetMathLibrary.MakeVector` (`KismetMathLibrary.Conv_IntToDouble` (* _returnvalue_2 -1)) (* _returnvalue_2 -1.5)))))
                (bind _returnvalue_3 (`|SpawnActorFromClass` "/Game/BearPressure/TileSystem/Sm_Road.Sm_Road_C" (`KismetMathLibrary.MakeTransform` (`KismetMathLibrary.MakeVector` _returnvalue_x (+ _returnvalue_y (`KismetMathLibrary.Conv_IntToDouble` (+ _road_lenght_2 (* (/ _array_element_2 2) _returnvalue_2)))) _returnvalue_z) (struct :`Yaw` 90.0)) "Undefined" "OverrideRootScale" null null))
                (`StaticMeshComponent.SetStaticMesh` (`StaticMeshActor.StaticMeshComponent` _returnvalue_3) (`|GetArrayItem` _road_tiles_2 (`KismetMathLibrary.RandomInteger` (`KismetArrayLibrary.Array_Length` _road_tiles_2))))))))))
    (:`then_1`
      (for _index_2 (range (+ (* (`self.Amount of roads in a row`) 2) 1))
        (`KismetArrayLibrary.Array_Clear` (`self.Temp Array`))
        (if (> (mod _index_2 2) 0)
          _
          (elif (not (`KismetArrayLibrary.Array_Contains` (`self.Road points X`) _index_2))
            (`KismetArrayLibrary.Array_Add` (`self.Temp Array`) _index_2)
            (for _array_element_3 (`self.Road Points Y`)
              (for _array_element_4 (`self.Temp Array`)
                (bind (_returnvalue_x_2 _returnvalue_y_2 _returnvalue_z_2) (`KismetMathLibrary.BreakVector` (+ (`KismetMathLibrary.MakeVector` 0.0 (`KismetMathLibrary.Conv_IntToDouble` (* _array_element_3 _road_lenght))) (`KismetMathLibrary.MakeVector` (* _returnvalue -1.5) (`KismetMathLibrary.Conv_IntToDouble` (* _returnvalue -1))))))
                (bind _returnvalue_4 (`|SpawnActorFromClass` "/Game/BearPressure/TileSystem/Sm_Road.Sm_Road_C" (`KismetMathLibrary.MakeTransform` (`KismetMathLibrary.MakeVector` (+ _returnvalue_x_2 (`KismetMathLibrary.Conv_IntToDouble` (+ _road_lenght (* (/ _array_element_4 2) _returnvalue)))) _returnvalue_y_2 _returnvalue_z_2)) "Undefined" "OverrideRootScale" null null))
                (`StaticMeshComponent.SetStaticMesh` (`StaticMeshActor.StaticMeshComponent` _returnvalue_4) (`|GetArrayItem` _road_tiles (`KismetMathLibrary.RandomInteger` (`KismetArrayLibrary.Array_Length` _road_tiles))))))))))))

(fn `UserConstructionScript`)